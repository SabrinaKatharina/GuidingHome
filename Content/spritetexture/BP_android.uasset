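; BP_android is a Paper2D character moved on X and Y input axes, with a directional walking sprite.
; Each axis event sets a single-axis Velocity from input and Speed, then moves CharacterMovement directly with sweep and calls the animation update.
; Both movement branches require the absolute axis value to exceed what reads as itself.
; The update picks idle or one of four walk flipbooks by Velocity's dominant axis and sign.
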(event Custom|update%20animation
  (bind _velocity (Variables|Default|Getvelocity))
  (bind (_x _y _z) (Math|Vector|BreakVector _velocity))
  ;[1 1 1] Update Flipbook Animation
  (Utilities|FlowControl|Sequence
    (:then_0
      (if (< (Math|Vector|VectorLengthSquared _velocity) 0.05)
        (Variables|Default|Setflipbook "/Game/spritetexture/idle.idle")
        (elif (> (Math|Float|Absolute(Float) _z) 0.0)
          (Variables|Default|Setflipbook "/Game/spritetexture/idle.idle")
          (elif (< (Math|Float|Absolute(Float) _x) (Math|Float|Absolute(Float) _y))
            ;;[1 1 1] y
            (if (< _y 0.0)
              (Variables|Default|Setflipbook "/Game/spritetexture/walk_back.walk_back")
              (else
                (Variables|Default|Setflipbook "/Game/spritetexture/walk_down.walk_down")))
            (else
              ;;[1 1 1] X-Axis
              (if (< _x 0.0)
                (Variables|Default|Setflipbook "/Game/spritetexture/walk_left.walk_left")
                (else
                  (Variables|Default|Setflipbook "/Game/spritetexture/walk_right.walk_right"))))))))
    (:then_1
      (Sprite|SetFlipbook (Variables|Default|GetSprite) (Variables|Default|Getflipbook)))))

(event Input|AxisEvents|InputAxisX
  (params (AxisValue :type Float%20%28single-precision%29))
  ;[1 1 1] Input X-Axis
  (Math|Float|CompareFloat (Math|Float|Absolute(Float) AxisValue) (Math|Float|Absolute(Float) (stale Input|AxisEvents|InputAxisY AxisValue))
    (:>
      (bind _output_get (Variables|Default|Setvelocity (Math|Vector|MakeVector (* AxisValue (Variables|Default|Getspeed)) 0.0 0.0)))
      (Class|MovementComponent|MoveUpdatedComponent (Variables|Character|GetCharacterMovement) _output_get "0, 0, 0" true)
      (CallFunction|UpdateAnimation))))

(event Input|AxisEvents|InputAxisY
  (params (AxisValue :type Float%20%28single-precision%29))
  ;[1 1 1] Input Y-Axis
  (Math|Float|CompareFloat (Math|Float|Absolute(Float) AxisValue) (Math|Float|Absolute(Float) (stale Input|AxisEvents|InputAxisX AxisValue))
    (:>
      (bind _output_get (Variables|Default|Setvelocity (Math|Vector|MakeVector 0.0 (* AxisValue (Variables|Default|Getspeed)) 0.0)))
      (Class|MovementComponent|MoveUpdatedComponent (Variables|Character|GetCharacterMovement) _output_get "0, 0, 0" true)
      (CallFunction|UpdateAnimation))))

(fn ConstructionScript
  (Variables|Default|Setspeed 1e+01))